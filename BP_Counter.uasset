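; BP_Counter is a score-counting actor that tallies BP_Pin actors entering its trigger box, likely for a bowling-style game.
; An overlap on Box destroys the pin, increments Score and writes the new value to the ScoreCounter text.
; A second trigger, Box1, plays the Pin_Cue sound at the world origin on any overlap, without checking which actor entered.
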(event OnComponentBeginOverlap(Box1)
  (params (OverlappedComponent :type Primitive%20Component%20Object%20Reference) (OtherActor :type Actor%20Object%20Reference) (OtherComp :type Primitive%20Component%20Object%20Reference) (OtherBodyIndex :type Integer) (bFromSweep :type Boolean) (SweepResult :type Hit%20Result%20Structure%20%28by%20ref%29))
  (Audio|PlaySoundatLocation "/Game/Assets/Audio/pin_Cue.pin_Cue" "0, 0, 0" "0, 0, 0" 1.0 1.0 0.0 0 0 0))

(event OnComponentBeginOverlap(Box)
  (params (OverlappedComponent :type Primitive%20Component%20Object%20Reference) (OtherActor :type Actor%20Object%20Reference) (OtherComp :type Primitive%20Component%20Object%20Reference) (OtherBodyIndex :type Integer) (bFromSweep :type Boolean) (SweepResult :type Hit%20Result%20Structure%20%28by%20ref%29))
  (if (== (Utilities|GetClass OtherActor) "/Game/Assets/Blueprints/BP_Pin.BP_Pin_C")
    (Actor|DestroyActor OtherActor)
    (bind _result (Math|Integer|IncrementInt (Variables|Default|GetScore))
      (:%20%20
        (Rendering|Components|TextRender|SetText (Variables|Default|GetScoreCounter) (Utilities|Text|ToText(String) (Utilities|String|Append "" (Utilities|String|ToString(Integer) _result))))))))

(event Collision|EventActorBeginOverlap
  (params (OtherActor :type Actor%20Object%20Reference)))

(event EventTick
  (params (DeltaSeconds :type Float%20%28single-precision%29)))

(fn ConstructionScript)