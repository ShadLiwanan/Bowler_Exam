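; BP_Player is a player Blueprint that aims and throws a ball along an arrow.
; The mouse wheel yaws the Arrow, and left click enables physics on the Ball and applies an impulse along the arrow's forward vector scaled by ThrowSpeed.
; A DoOnce limits the throw to a single firing.
; R reopens the Main level and also wires into that DoOnce.
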(event Input|MouseEvents|MouseWheelAxis
  (params (AxisValue :type Float%20%28single-precision%29))
  (Transformation|AddLocalRotation (Variables|Default|GetArrow) (Math|Rotator|MakeRotator 0.0 0.0 AxisValue) false false))

(event Input|MouseEvents|LeftMouseButton
  (params (Key :type Key%20Structure :default "None"))
  (bind _ball (Variables|Default|GetBall))
  (:Pressed
    (Utilities|FlowControl|DoOnce false
      (:Completed
        (Physics|SetSimulatePhysics _ball true)
        (Physics|AddImpulse _ball (* (Math|Vector|GetForwardVector (Variables|Default|GetArrow)) (Variables|Default|GetThrowSpeed)) "None" false)))))

(event Input|KeyboardEvents|R
  (params (Key :type Key%20Structure :default "None"))
  (bind _ball (Variables|Default|GetBall))
  (:Pressed
    (Game|OpenLevel(byName) "Main")
    (Utilities|FlowControl|DoOnce false
      (:Completed
        (Physics|SetSimulatePhysics _ball true)
        (Physics|AddImpulse _ball (* (Math|Vector|GetForwardVector (Variables|Default|GetArrow)) (Variables|Default|GetThrowSpeed)) "None" false)))))

(fn ConstructionScript)